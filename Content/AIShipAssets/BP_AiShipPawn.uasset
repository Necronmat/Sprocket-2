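; AI ship pawn that displays its hull and shield status on a HealthBar widget.
; Every Tick forces the bar visible, then casts the controller to BB_AIShipController and passes its current and max hull and shield values to the widget through interface messages.
; An unconnected player distance and dot-product check is left in the graph, so visibility is never conditional.
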(event EventBeginPlay)

(event Collision|EventActorBeginOverlap
  (params (OtherActor :type Actor%20Object%20Reference)))

(event EventTick
  (params (DeltaSeconds :type Float%20%28single-precision%29))
  (Class|BPIShipHealthBarVisibility|SetHealthBarVisibility(Message) (UserInterface|GetUserWidgetObject (Variables|Default|GetHealthBar)) true)
  (bind _asbb_aiship_controller (Utilities|Casting|CastToBB_AIShipController (Pawn|GetController)))
  (Class|BPIShipHealthBarVisibility|SetHealthBarValue(Message) (UserInterface|GetUserWidgetObject (Variables|Default|GetHealthBar)) (Class|AIShipController|GetCurrentHull _asbb_aiship_controller) (Class|AIShipController|GetMaxHull _asbb_aiship_controller) (Class|AIShipController|GetCurrentShield _asbb_aiship_controller) (Class|AIShipController|GetMaxShield _asbb_aiship_controller)))

(fn ConstructionScript)